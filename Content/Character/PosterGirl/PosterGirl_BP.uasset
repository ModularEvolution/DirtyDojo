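; PosterGirl is a character display Blueprint that shows mesh animations with physics-driven breast jiggle.
; On BeginPlay it applies constraint and physical animation profiles, then simulates bodies below both breast bones on the skeletal mesh.
; The Animswitch timeline's event tracks switch between CP, idle, leg-hit and head-hit animations.
; A box overlap prints a debug "Hello" and plays the head-hit animation once.
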(event OnComponentBeginOverlap(Box)
  (params (OverlappedComponent :type Primitive%20Component%20Object%20Reference) (OtherActor :type Actor%20Object%20Reference) (OtherComp :type Primitive%20Component%20Object%20Reference) (OtherBodyIndex :type Integer) (bFromSweep :type Boolean) (SweepResult :type Hit%20Result%20Structure%20%28by%20ref%29))
  (Development|PrintString "Hello")
  (Components|Animation|PlayAnimation (Variables|Default|GetSkeletalMesh) "/Game/Character/PosterGirl/mediumHitHeadMeshOnly_Anim.mediumHitHeadMeshOnly_Anim" false))

(event EventBeginPlay
  (bind _physicalanimation (Variables|Default|GetPhysicalAnimation))
  (bind _skeletalmesh (Variables|Default|GetSkeletalMesh))
  (bind _rboob (Variables|Default|GetRBoob))
  (bind _lboob (Variables|Default|GetLBoob))
  (bind _skeletalmesh_2 (Variables|Default|GetSkeletalMesh))
  (Class|PhysicalAnimationComponent|SetSkeletalMeshComponent _physicalanimation _skeletalmesh)
  (Class|SkeletalMeshComponent|SetConstraintProfileforAll _skeletalmesh "Test_Constr" false)
  (Class|PhysicalAnimationComponent|ApplyPhysicalAnimationProfileBelow _physicalanimation _lboob "Test_PAnim" true false)
  (Class|PhysicalAnimationComponent|ApplyPhysicalAnimationProfileBelow _physicalanimation _rboob "Test_PAnim" true false)
  (Class|SkeletalMeshComponent|SetAllBodiesBelowSimulatePhysics _skeletalmesh _lboob true true)
  (Class|SkeletalMeshComponent|SetAllBodiesBelowSimulatePhysics _skeletalmesh _rboob true true)
  (Timeline|animswitch Play
    (:New_Track_0
      (Components|Animation|SetAnimation _skeletalmesh_2 "/Game/Character/PosterGirl/CP_MeshOnly_Anim.CP_MeshOnly_Anim"))
    (:NewTrack_1
      (Components|Animation|SetAnimation _skeletalmesh_2 "/Game/Character/PosterGirl/idle_MeshOnly_Anim.idle_MeshOnly_Anim"))
    (:NewTrack_2
      (Components|Animation|SetAnimation _skeletalmesh_2 "/Game/Character/PosterGirl/LegHitMeshOnly_Anim.LegHitMeshOnly_Anim"))
    (:NewTrack_3
      (Components|Animation|SetAnimation _skeletalmesh_2 "/Game/Character/PosterGirl/mediumHitHeadMeshOnly_Anim.mediumHitHeadMeshOnly_Anim")))
  (Audio|Components|Audio|Play _skeletalmesh_2 true))

(event Collision|EventActorBeginOverlap
  (params (OtherActor :type Actor%20Object%20Reference)))

(event EventTick
  (params (DeltaSeconds :type Float%20%28single-precision%29)))

(fn ConstructionScript)