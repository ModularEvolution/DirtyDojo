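; Fight manager actor that sets up and referees a one-on-one fight, spawning two pawns, possessing the left, and creating the fight UI.
; Tick polls and relays hit and damage flags between pawns, and pushes HP, left-player stress and "river" array updates to widgets.
; Shout buttons trigger left-pawn moves; all except Guard add stress cost, and all are marked unavailable near the stress cap.
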(event Custom|UpdateRiver
  (bind _fightui (Variables|Default|GetFightUI))
  (bind _player_right (Variables|Default|GetPlayer_Right))
  (bind _player_left (Variables|Default|GetPlayer_Left))
  (bind _riverhoriz_left_wdg (Variables|/Game/UI/FightUI/FightUI_WDG.FightUI_WDG_C|GetRiverHoriz_Left_WDG _fightui))
  (bind _riverhoriz_right_wdg (Variables|/Game/UI/FightUI/FightUI_WDG.FightUI_WDG_C|GetRiverHoriz_Right_WDG _fightui))
  (if (Variables|/Game/Blueprints/PG_Pawn_v4_BP.PG_Pawn_v4_BP_C|GetUpdateRiver _player_left)
    (Variables|/Game/Blueprints/PG_Pawn_v4_BP.PG_Pawn_v4_BP_C|SetUpdateRiver _player_left false)
    (Variables|/Game/UI/FightUI/RiverHoriz_WDG.RiverHoriz_WDG_C|SetRiverArray _riverhoriz_left_wdg (Variables|/Game/Blueprints/PG_Pawn_v4_BP.PG_Pawn_v4_BP_C|GetRiverElemArray _player_left))
    (Default|UpdateRiver _riverhoriz_left_wdg)
    (else
      (Variables|/Game/Blueprints/PG_Pawn_v4_BP.PG_Pawn_v4_BP_C|SetUpdateRiver _player_right false)
      (Variables|/Game/UI/FightUI/RiverHoriz_WDG.RiverHoriz_WDG_C|SetRiverArray _riverhoriz_right_wdg (Variables|/Game/Blueprints/PG_Pawn_v4_BP.PG_Pawn_v4_BP_C|GetRiverElemArray _player_right))
      (Default|UpdateRiver _riverhoriz_right_wdg))))

(event EventBeginPlay
  (bind _returnvalue (Game|GetPlayerController 0))
  (bind _returnvalue_2 (Transformation|GetActorLocation))
  (bind _returnvalue_3 (Transformation|GetActorLocation))
  (bind _returnvalue_4 (Game|SpawnActorfromClass "/Game/Blueprints/PG_Pawn_v4_BP.PG_Pawn_v4_BP_C" (Math|Transform|MakeTransform (Math|Vector|MakeVector (- (.x _returnvalue_3) 3e+01) (.y _returnvalue_3) (.z _returnvalue_3)) "0, 0, 0" "1,1,1") "Undefined" (Game|GetPlayerController 0) 0))
  (bind _output_get (Variables|Default|SetPlayer_Left _returnvalue_4))
  (Pawn|Possess (Game|GetPlayerController 0) _output_get)
  (bind _returnvalue_5 (Game|SpawnActorfromClass "/Game/Blueprints/PG_Pawn_v4_BP.PG_Pawn_v4_BP_C" (Math|Transform|MakeTransform (Math|Vector|MakeVector (+ (.x _returnvalue_2) 35.0) (- (.y _returnvalue_2) 5.0) (.z _returnvalue_2)) "0,180.000000, 0" "1,1,1") "Undefined" (Game|GetPlayerController 0) 0))
  (Variables|Default|SetPlayer_Right _returnvalue_5)
  (bind _returnvalue_6 (UserInterface|CreateWidget "/Game/UI/FightUI/FightUI_WDG.FightUI_WDG_C" (Game|GetPlayerController 0)))
  (bind _output_get_2 (Variables|Default|SetFightUI _returnvalue_6))
  (UserInterface|Viewport|AddtoViewport _output_get_2 0)
  (Input|SetInputModeGameandUI _returnvalue _output_get_2 "DoNotLock" true)
  (Variables|/Script/Engine.PlayerController|SetbShowMouseCursor _returnvalue true)
  (Variables|/Game/UI/FightUI/FightUI_WDG.FightUI_WDG_C|SetPlayerLeftStressPoolMax (Variables|Default|GetFightUI) (Variables|/Game/Blueprints/PG_Pawn_v4_BP.PG_Pawn_v4_BP_C|GetStressPoolMax (Variables|Default|GetPlayer_Left)))
  (Variables|/Game/UI/FightUI/FightUI_WDG.FightUI_WDG_C|SetPL_HPMax (Variables|Default|GetFightUI) (Variables|/Game/Blueprints/PG_Pawn_v4_BP.PG_Pawn_v4_BP_C|GetHPMax (Variables|Default|GetPlayer_Left)))
  (Variables|/Game/UI/FightUI/FightUI_WDG.FightUI_WDG_C|SetPR_HPMax (Variables|Default|GetFightUI) (Variables|/Game/Blueprints/PG_Pawn_v4_BP.PG_Pawn_v4_BP_C|GetHPMax (Variables|Default|GetPlayer_Right))))

(event Collision|EventActorBeginOverlap
  (params (OtherActor :type Actor%20Object%20Reference)))

(event EventTick
  (params (DeltaSeconds :type Float%20%28single-precision%29))
  (bind _player_left (Variables|Default|GetPlayer_Left))
  (bind _player_left_2 (Variables|Default|GetPlayer_Left))
  (bind _player_right (Variables|Default|GetPlayer_Right))
  (bind _player_right_2 (Variables|Default|GetPlayer_Right))
  (bind _fightui (Variables|Default|GetFightUI))
  (bind _player_left_3 (Variables|Default|GetPlayer_Left))
  (bind _player_left_4 (Variables|Default|GetPlayer_Left))
  (bind _fightui_2 (Variables|Default|GetFightUI))
  (bind _shoutbtn_wdg_powerattack (Variables|/Game/UI/FightUI/FightUI_WDG.FightUI_WDG_C|GetShoutBtn_WDG_PowerAttack _fightui))
  (bind _shoutbtn_wdg_punch (Variables|/Game/UI/FightUI/FightUI_WDG.FightUI_WDG_C|GetShoutBtn_WDG_Punch _fightui))
  (bind _shoutbtn_wdg_kick (Variables|/Game/UI/FightUI/FightUI_WDG.FightUI_WDG_C|GetShoutBtn_WDG_Kick _fightui))
  (bind _shoutbtn_wdg_guard (Variables|/Game/UI/FightUI/FightUI_WDG.FightUI_WDG_C|GetShoutBtn_WDG_Guard _fightui))
  (Variables|/Game/Blueprints/PG_Pawn_v4_BP.PG_Pawn_v4_BP_C|SetGetHit (Variables|Default|GetPlayer_Right) (Variables|/Game/Blueprints/PG_Pawn_v4_BP.PG_Pawn_v4_BP_C|GetApplyHit _player_left_4))
  (Variables|/Game/Blueprints/PG_Pawn_v4_BP.PG_Pawn_v4_BP_C|SetApplyHit _player_left_4 false)
  (Variables|/Game/Blueprints/PG_Pawn_v4_BP.PG_Pawn_v4_BP_C|SetGetHit (Variables|Default|GetPlayer_Left) (Variables|/Game/Blueprints/PG_Pawn_v4_BP.PG_Pawn_v4_BP_C|GetApplyHit _player_right))
  (Variables|/Game/Blueprints/PG_Pawn_v4_BP.PG_Pawn_v4_BP_C|SetApplyHit _player_right false)
  (Variables|/Game/Blueprints/PG_Pawn_v4_BP.PG_Pawn_v4_BP_C|SetGetHitBreak _player_right_2 (Variables|/Game/Blueprints/PG_Pawn_v4_BP.PG_Pawn_v4_BP_C|GetActionPowerAttack _player_left_2))
  (if (or (Variables|/Game/Blueprints/PG_Pawn_v4_BP.PG_Pawn_v4_BP_C|GetUpdateRiver _player_right_2) (Variables|/Game/Blueprints/PG_Pawn_v4_BP.PG_Pawn_v4_BP_C|GetUpdateRiver _player_left_2))
    (CallFunction|UpdateRiver))
  (Variables|/Game/Blueprints/PG_Pawn_v4_BP.PG_Pawn_v4_BP_C|SetDmgReceived (Variables|Default|GetPlayer_Right) (Variables|/Game/Blueprints/PG_Pawn_v4_BP.PG_Pawn_v4_BP_C|GetDmgGiven (Variables|Default|GetPlayer_Left)))
  (Variables|/Game/Blueprints/PG_Pawn_v4_BP.PG_Pawn_v4_BP_C|SetDmgReceived (Variables|Default|GetPlayer_Left) (Variables|/Game/Blueprints/PG_Pawn_v4_BP.PG_Pawn_v4_BP_C|GetDmgGiven (Variables|Default|GetPlayer_Right)))
  (Variables|/Game/UI/FightUI/FightUI_WDG.FightUI_WDG_C|SetPlayerLeftStressPool _fightui_2 (Variables|/Game/Blueprints/PG_Pawn_v4_BP.PG_Pawn_v4_BP_C|GetStressPool _player_left))
  (CallFunction|IsStressAvailable _fightui_2 _player_left)
  (Variables|/Game/UI/FightUI/FightUI_WDG.FightUI_WDG_C|SetPL_HP (Variables|Default|GetFightUI) (Variables|/Game/Blueprints/PG_Pawn_v4_BP.PG_Pawn_v4_BP_C|GetHP (Variables|Default|GetPlayer_Left)))
  (Variables|/Game/UI/FightUI/FightUI_WDG.FightUI_WDG_C|SetPR_HP (Variables|Default|GetFightUI) (Variables|/Game/Blueprints/PG_Pawn_v4_BP.PG_Pawn_v4_BP_C|GetHP (Variables|Default|GetPlayer_Right)))
  (Utilities|FlowControl|Sequence
    (:then_0
      (if (Variables|/Game/UI/FightUI/ShoutBtn_WDG.ShoutBtn_WDG_C|GetShoutPressed _shoutbtn_wdg_punch)
        (Default|ShoutPunch _player_left_3)
        (Variables|/Game/UI/FightUI/ShoutBtn_WDG.ShoutBtn_WDG_C|SetShoutPressed _shoutbtn_wdg_punch false)
        (CallFunction|UpdateStress _player_left_3 _shoutbtn_wdg_punch)))
    (:then_1
      (if (Variables|/Game/UI/FightUI/ShoutBtn_WDG.ShoutBtn_WDG_C|GetShoutPressed _shoutbtn_wdg_kick)
        (Default|ShoutKick _player_left_3)
        (Variables|/Game/UI/FightUI/ShoutBtn_WDG.ShoutBtn_WDG_C|SetShoutPressed _shoutbtn_wdg_kick false)
        (CallFunction|UpdateStress _player_left_3 _shoutbtn_wdg_kick)))
    (:then_2
      (if (Variables|/Game/UI/FightUI/ShoutBtn_WDG.ShoutBtn_WDG_C|GetShoutPressed _shoutbtn_wdg_guard)
        (Default|ShoutBlock _player_left_3)
        (Variables|/Game/UI/FightUI/ShoutBtn_WDG.ShoutBtn_WDG_C|SetShoutPressed _shoutbtn_wdg_guard false)))
    (:then_3
      (if (Variables|/Game/UI/FightUI/ShoutBtn_WDG.ShoutBtn_WDG_C|GetShoutPressed _shoutbtn_wdg_powerattack)
        (Default|ShoutPowerAttack _player_left_3)
        (Variables|/Game/UI/FightUI/ShoutBtn_WDG.ShoutBtn_WDG_C|SetShoutPressed _shoutbtn_wdg_powerattack false)
        (CallFunction|UpdateStress _player_left_3 _shoutbtn_wdg_powerattack)))))

(fn ConstructionScript)

(fn UpdateStress
  (params (PlayerRef :type PG%20Pawn%20V%204%20BP%20Object%20Reference) (ShoutButtonRef :type Shout%20Btn%20WDG%20Object%20Reference))
  (Variables|/Game/Blueprints/PG_Pawn_v4_BP.PG_Pawn_v4_BP_C|SetStressPool PlayerRef (+ (Variables|/Game/Blueprints/PG_Pawn_v4_BP.PG_Pawn_v4_BP_C|GetStressPool PlayerRef) (Variables|/Game/UI/FightUI/ShoutBtn_WDG.ShoutBtn_WDG_C|GetShoutCost ShoutButtonRef))))

(fn IsStressAvailable
  (params (FightUI :type Fight%20UI%20WDG%20Object%20Reference) (PlayerRef :type PG%20Pawn%20V%204%20BP%20Object%20Reference))
  (bind _shoutbtn_wdg_powerattack (Variables|/Game/UI/FightUI/FightUI_WDG.FightUI_WDG_C|GetShoutBtn_WDG_PowerAttack FightUI))
  (bind _shoutbtn_wdg_guard (Variables|/Game/UI/FightUI/FightUI_WDG.FightUI_WDG_C|GetShoutBtn_WDG_Guard FightUI))
  (bind _shoutbtn_wdg_kick (Variables|/Game/UI/FightUI/FightUI_WDG.FightUI_WDG_C|GetShoutBtn_WDG_Kick FightUI))
  (bind _shoutbtn_wdg_punch (Variables|/Game/UI/FightUI/FightUI_WDG.FightUI_WDG_C|GetShoutBtn_WDG_Punch FightUI))
  (if (< (Variables|/Game/Blueprints/PG_Pawn_v4_BP.PG_Pawn_v4_BP_C|GetStressPool PlayerRef) (- (Variables|/Game/Blueprints/PG_Pawn_v4_BP.PG_Pawn_v4_BP_C|GetStressPoolMax PlayerRef) 5.0))
    (Variables|/Game/UI/FightUI/ShoutBtn_WDG.ShoutBtn_WDG_C|SetStressAvailable _shoutbtn_wdg_guard true)
    (Variables|/Game/UI/FightUI/ShoutBtn_WDG.ShoutBtn_WDG_C|SetStressAvailable _shoutbtn_wdg_kick true)
    (Variables|/Game/UI/FightUI/ShoutBtn_WDG.ShoutBtn_WDG_C|SetStressAvailable _shoutbtn_wdg_punch true)
    (Variables|/Game/UI/FightUI/ShoutBtn_WDG.ShoutBtn_WDG_C|SetStressAvailable _shoutbtn_wdg_powerattack true)
    (else
      (Variables|/Game/UI/FightUI/ShoutBtn_WDG.ShoutBtn_WDG_C|SetStressAvailable _shoutbtn_wdg_guard false)
      (Variables|/Game/UI/FightUI/ShoutBtn_WDG.ShoutBtn_WDG_C|SetStressAvailable _shoutbtn_wdg_kick false)
      (Variables|/Game/UI/FightUI/ShoutBtn_WDG.ShoutBtn_WDG_C|SetStressAvailable _shoutbtn_wdg_punch false)
      (Variables|/Game/UI/FightUI/ShoutBtn_WDG.ShoutBtn_WDG_C|SetStressAvailable _shoutbtn_wdg_powerattack false))))