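; Player pawn for a fighting game that turns punch, kick, block and power attack "shouts" into actions appended to ActionRiver.
; Input actions and custom Shout events share the same paths for punch, kick and block, while power attack has only an event.
; BeginPlay starts physics simulation on the hair bones and adds the fight UI to the viewport.
; CheckHitCol sets ApplyHit when another actor's HitCol or HeadCol component is matched by name.
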(event Custom|ShoutPunch
  ;[1 0.008376 0] Shout Inputs TODO: Add action as first in river
  (bind _returnvalue (Class|Fighter|ShoutAction "Punch"))
  (Utilities|Array|Add (Variables|Default|GetactionRiver) _returnvalue))

(event Custom|ShoutPowerAttack
  ;[1 0.008376 0] Shout Inputs TODO: Add action as first in river
  (bind _returnvalue (Class|Fighter|ShoutAction "PowerAttack"))
  (Utilities|Array|Add (Variables|Default|GetactionRiver) _returnvalue))

(event Custom|ShoutKick
  ;[1 0.008376 0] Shout Inputs TODO: Add action as first in river
  (bind _returnvalue (Class|Fighter|ShoutAction "Kick"))
  (Utilities|Array|Add (Variables|Default|GetactionRiver) _returnvalue))

(event Custom|ShoutBlock
  ;[1 0.008376 0] Shout Inputs TODO: Add action as first in river
  (bind _returnvalue (Class|Fighter|ShoutAction "Block"))
  (Utilities|Array|Add (Variables|Default|GetactionRiver) _returnvalue))

(event EventBeginPlay
  ;[1 0.507 0] Set Hair Simulation TODO: Move it to C++
  (Class|PhysicalAnimationComponent|SetSkeletalMeshComponent (Variables|Default|GetPhysicalAnimation) (Variables|Default|GetHair))
  (Class|SkeletalMeshComponent|SetAllBodiesBelowSimulatePhysics (Variables|Default|GetHair) (Variables|Default|GetHairJoint2Simulate) true true)
  (bind _returnvalue (UserInterface|CreateWidget "/Game/UI/C++FIghtUI/FightUI_WDG_2.FightUI_WDG_2_C"))
  (UserInterface|Viewport|AddtoViewport _returnvalue 0))

(event Input|ActionEvents|InputActionPunch_1
  (params (Key :type Key%20Structure))
  ;[1 0.008376 0] Shout Inputs TODO: Add action as first in river
  (:Pressed
    (bind _returnvalue (Class|Fighter|ShoutAction "Punch"))
    (Utilities|Array|Add (Variables|Default|GetactionRiver) _returnvalue)))

(event Input|ActionEvents|InputActionGuard_3
  (params (Key :type Key%20Structure))
  ;[1 0.008376 0] Shout Inputs TODO: Add action as first in river
  (:Pressed
    (bind _returnvalue (Class|Fighter|ShoutAction "Block"))
    (Utilities|Array|Add (Variables|Default|GetactionRiver) _returnvalue)))

(event Input|ActionEvents|InputActionKick_2
  (params (Key :type Key%20Structure))
  ;[1 0.008376 0] Shout Inputs TODO: Add action as first in river
  (:Pressed
    (bind _returnvalue (Class|Fighter|ShoutAction "Kick"))
    (Utilities|Array|Add (Variables|Default|GetactionRiver) _returnvalue)))

(fn ConstructionScript)

(fn CheckHitCol
  (params (OtherActor :type Object%20Object%20Reference) (AtherComponent :type Object%20Object%20Reference))
  (bind _returnvalue (Utilities|GetObjectName AtherComponent))
  (if (not (== OtherActor self))
    (if (or (Utilities|Enum|Equal(Enum) _returnvalue "HitCol") (Utilities|Enum|Equal(Enum) _returnvalue "HeadCol"))
      (Variables|Default|SetApplyHit true))))