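; Fighting-game pawn that carries out punches, kicks, parries, blocks and power attacks from a queue called the River.
; DecideAction refills the River with random moves, while shouts from input or events insert moves at its front.
; A looping DoAction timer turns queue entries into action flags and damage, gated by attack/defence completion.
; Overlap colliders flag hits, HitReceived reduces HP, a timer drains StressPool, and hair uses physics simulation.
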(event OnComponentBeginOverlap(HandCol)
  (params (OverlappedComponent :type Primitive%20Component%20Object%20Reference) (OtherActor :type Actor%20Object%20Reference) (OtherComp :type Primitive%20Component%20Object%20Reference) (OtherBodyIndex :type Integer) (bFromSweep :type Boolean) (SweepResult :type Hit%20Result%20Structure%20%28by%20ref%29))
  ;[1 1 1] Collision Handling
  (CallFunction|CheckHitCol OtherActor OtherComp))

(event OnComponentBeginOverlap(FootCol)
  (params (OverlappedComponent :type Primitive%20Component%20Object%20Reference) (OtherActor :type Actor%20Object%20Reference) (OtherComp :type Primitive%20Component%20Object%20Reference) (OtherBodyIndex :type Integer) (bFromSweep :type Boolean) (SweepResult :type Hit%20Result%20Structure%20%28by%20ref%29))
  ;[1 1 1] Collision Handling
  (CallFunction|CheckHitCol OtherActor OtherComp))

(event OnComponentBeginOverlap(HitCol)
  (params (OverlappedComponent :type Primitive%20Component%20Object%20Reference) (OtherActor :type Actor%20Object%20Reference) (OtherComp :type Primitive%20Component%20Object%20Reference) (OtherBodyIndex :type Integer) (bFromSweep :type Boolean) (SweepResult :type Hit%20Result%20Structure%20%28by%20ref%29))
  ;[1 1 1] Collision Handling
  (CallFunction|CheckHitCol OtherActor OtherComp))

(event OnComponentBeginOverlap(HeadCol)
  (params (OverlappedComponent :type Primitive%20Component%20Object%20Reference) (OtherActor :type Actor%20Object%20Reference) (OtherComp :type Primitive%20Component%20Object%20Reference) (OtherBodyIndex :type Integer) (bFromSweep :type Boolean) (SweepResult :type Hit%20Result%20Structure%20%28by%20ref%29))
  ;[1 1 1] Collision Handling
  (CallFunction|CheckHitCol OtherActor OtherComp))

(event Custom|ShoutPunch
  ;[1 1 1] Shout Inputs
  (Variables|Default|SetShouted_Action "Punch")
  (Utilities|Array|Insert (Variables|Default|GetRiverElemArray) (Variables|Default|GetShouted_Action))
  (Variables|Default|SetShout true)
  (Rendering|Components|TextRender|SetText (Variables|Default|GetTextRender) (Utilities|Text|ToText(String) (Variables|Default|GetShouted_Action)))
  (Variables|Default|SetUpdateRiver true)
  (CallFunction|DoAction))

(event Custom|ShoutPowerAttack
  ;[1 1 1] Shout Inputs
  (Variables|Default|SetShouted_Action "PowerAttack")
  (Utilities|Array|Insert (Variables|Default|GetRiverElemArray) (Variables|Default|GetShouted_Action))
  (Variables|Default|SetShout true)
  (Rendering|Components|TextRender|SetText (Variables|Default|GetTextRender) (Utilities|Text|ToText(String) (Variables|Default|GetShouted_Action)))
  (Variables|Default|SetUpdateRiver true)
  (CallFunction|DoAction))

(event Custom|StaminaGain
  ;[1 1 1] Stress pool Gain
  (if (> (Variables|Default|GetStressPool) (Variables|Default|GetStaminaRegen))
    (Variables|Default|SetStressPool (- (Variables|Default|GetStressPool) (Variables|Default|GetStaminaRegen)))))

(event Custom|DecideAction
  (bind _riverelemarray (Variables|Default|GetRiverElemArray))
  (bind _returnvalue (Utilities|Array|Length _riverelemarray))
  (if (Pawn|IsPlayerControlled)
    _
    (else
      _))
  (if (<= _returnvalue 3)
    (for _index (range (- _returnvalue 1) 2)
      ;[1 1 1] Decide Next Action
      (switch int (Math|Random|RandomInteger 2)
        (:0
          (switch int (Math|Random|RandomInteger 2)
            (:0
              (Variables|Default|SetDoActionName "Punch"))
            (:1
              (Variables|Default|SetDoActionName "Kick"))))
        (:1
          (switch int (Math|Random|RandomInteger 2)
            (:0
              (Variables|Default|SetDoActionName "Parry"))
            (:1
              (Variables|Default|SetDoActionName "Block"))))
        (:2
          (Variables|Default|SetDoActionName "Idle")))
      (Utilities|Array|Add (Variables|Default|GetRiverElemArray) (Variables|Default|GetDoActionName)))
    (Variables|Default|SetUpdateRiver true)))

(event Custom|ShoutKick
  ;[1 1 1] Shout Inputs
  (Variables|Default|SetShouted_Action "Kick")
  (Utilities|Array|Insert (Variables|Default|GetRiverElemArray) (Variables|Default|GetShouted_Action))
  (Variables|Default|SetShout true)
  (Rendering|Components|TextRender|SetText (Variables|Default|GetTextRender) (Utilities|Text|ToText(String) (Variables|Default|GetShouted_Action)))
  (Variables|Default|SetUpdateRiver true)
  (CallFunction|DoAction))

(event Custom|ShoutBlock
  ;[1 1 1] Shout Inputs
  (Variables|Default|SetShouted_Action "Block")
  (Utilities|Array|Insert (Variables|Default|GetRiverElemArray) (Variables|Default|GetShouted_Action))
  (Variables|Default|SetShout true)
  (Rendering|Components|TextRender|SetText (Variables|Default|GetTextRender) (Utilities|Text|ToText(String) (Variables|Default|GetShouted_Action)))
  (Variables|Default|SetUpdateRiver true)
  (CallFunction|DoAction))

(event Custom|DoAction
  ;[1 1 1] Do Action ( AI decided or Shout )
  (if (and (Variables|Default|GetFinishedAttack) (Variables|Default|GetFinishedDefence))
    (Utilities|Array|RemoveIndex (Variables|Default|GetRiverElemArray))
    (Variables|Default|SetUpdateRiver true :!label _label)
    (switch string (Utilities|Array|Get(acopy) (Variables|Default|GetRiverElemArray))
      (:Punch
        (Variables|Actions|SetActionPunch true)
        (Variables|Default|SetDmgGiven (Variables|Default|GetDmgPunch))
        (Variables|Default|SetFinishedAttack false :!label _label_2))
      (:Kick
        (Variables|Actions|SetActionKick true)
        (Variables|Default|SetDmgGiven (Variables|Default|GetDmgKick))
        (goto _label_2))
      (:Parry
        (Variables|Actions|SetActionParry true)
        (Variables|Default|SetFinishedDefence false :!label _label_3))
      (:Block
        (Variables|Actions|SetActionBlock true)
        (goto _label_3))
      (:Idle
        (Variables|Actions|SetActionIdle true))
      (:PowerAttack
        (Variables|Actions|SetActionKick true)
        (Variables|Actions|SetActionPowerAttack true)
        (Variables|Default|SetDmgGiven (Variables|Default|GetDmgPwrAttack))
        (goto _label_2)))
    (Rendering|Components|TextRender|SetText (Variables|Default|GetTextRender) (Utilities|Text|ToText(String) (Utilities|Array|Get(acopy) (Variables|Default|GetRiverElemArray))))
    (CallFunction|DecideAction)
    (elif (and (Variables|Default|GetShout) (Variables|Default|GetFinishedAttack))
      (goto _label))))

(event Custom|HitReceived
  ;[1 1 1] Received Hit - Counting it
  (Variables|Default|SetHP (- (Variables|Default|GetHP) (Variables|Default|GetDmgReceived))))

(event EventBeginPlay
  ;[1 1 1] Begin Play - Start timers, Set Stamina
  (CallFunction|DecideAction)
  (Utilities|Time|SetTimerbyFunctionName 0 "DoAction" 2.0 true)
  (Utilities|Time|SetTimerbyFunctionName 0 "StaminaGain" 1.0 true)
  (Variables|Default|SetHP (Variables|Default|GetHPMax))
  ;[1 1 1] Set Hair Simulation
  (Class|PhysicalAnimationComponent|SetSkeletalMeshComponent (Variables|Default|GetPhysicalAnimation) (Variables|Default|GetHair))
  (Class|SkeletalMeshComponent|SetAllBodiesBelowSimulatePhysics (Variables|Default|GetHair) (Variables|Default|GetHairJoint2Simulate) true true))

(event EventTick
  (params (DeltaSeconds :type Float%20%28single-precision%29))
  ;[1 1 1] Event Tick : Update states
  (Utilities|FlowControl|Sequence
    (:then_0
      (if (Variables|Default|GetFinishedAttack)
        (Variables|Actions|SetActionPunch false)
        (Variables|Actions|SetActionKick false)
        (Variables|Actions|SetActionPowerAttack false)))
    (:then_1
      (if (Variables|Default|GetFinishedDefence)
        (Variables|Actions|SetActionParry false)
        (Variables|Actions|SetActionBlock false)))))

(event Input|ActionEvents|InputActionPunch_1
  (params (Key :type Key%20Structure))
  ;[1 1 1] Shout Inputs
  (:Pressed
    (Variables|Default|SetShouted_Action "Punch")
    (Utilities|Array|Insert (Variables|Default|GetRiverElemArray) (Variables|Default|GetShouted_Action))
    (Variables|Default|SetShout true)
    (Rendering|Components|TextRender|SetText (Variables|Default|GetTextRender) (Utilities|Text|ToText(String) (Variables|Default|GetShouted_Action)))
    (Variables|Default|SetUpdateRiver true)
    (CallFunction|DoAction)))

(event Input|ActionEvents|InputActionGuard_3
  (params (Key :type Key%20Structure))
  ;[1 1 1] Shout Inputs
  (:Pressed
    (Variables|Default|SetShouted_Action "Block")
    (Utilities|Array|Insert (Variables|Default|GetRiverElemArray) (Variables|Default|GetShouted_Action))
    (Variables|Default|SetShout true)
    (Rendering|Components|TextRender|SetText (Variables|Default|GetTextRender) (Utilities|Text|ToText(String) (Variables|Default|GetShouted_Action)))
    (Variables|Default|SetUpdateRiver true)
    (CallFunction|DoAction)))

(event Input|ActionEvents|InputActionKick_2
  (params (Key :type Key%20Structure))
  ;[1 1 1] Shout Inputs
  (:Pressed
    (Variables|Default|SetShouted_Action "Kick")
    (Utilities|Array|Insert (Variables|Default|GetRiverElemArray) (Variables|Default|GetShouted_Action))
    (Variables|Default|SetShout true)
    (Rendering|Components|TextRender|SetText (Variables|Default|GetTextRender) (Utilities|Text|ToText(String) (Variables|Default|GetShouted_Action)))
    (Variables|Default|SetUpdateRiver true)
    (CallFunction|DoAction)))

(fn ConstructionScript)

(fn CheckHitCol
  (params (OtherActor :type Object%20Object%20Reference) (AtherComponent :type Object%20Object%20Reference))
  (bind _returnvalue (Utilities|GetObjectName AtherComponent))
  (if (not (== OtherActor self))
    (if (or (Utilities|Enum|Equal(Enum) _returnvalue "HitCol") (Utilities|Enum|Equal(Enum) _returnvalue "HeadCol"))
      (Variables|Default|SetApplyHit true))))