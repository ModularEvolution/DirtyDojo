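; Fighter pawn that randomly punches, kicks, parries, blocks or idles, while a controlling player can shout commands to steer it.
; A looping DecideAction timer picks actions, giving shouts priority but holding them until attacks finish, and DoAction sets state flags, damage and text labels.
; Limb and body collision overlaps flag hits, and HitReceived subtracts HP.
; A second timer drains the stress pool, and hair simulates physics below a joint.
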(event OnComponentBeginOverlap(HandCol)
  (params (OverlappedComponent :type Primitive%20Component%20Object%20Reference) (OtherActor :type Actor%20Object%20Reference) (OtherComp :type Primitive%20Component%20Object%20Reference) (OtherBodyIndex :type Integer) (bFromSweep :type Boolean) (SweepResult :type Hit%20Result%20Structure%20%28by%20ref%29))
  (CallFunction|CheckHitCol OtherActor OtherComp))

(event OnComponentBeginOverlap(FootCol)
  (params (OverlappedComponent :type Primitive%20Component%20Object%20Reference) (OtherActor :type Actor%20Object%20Reference) (OtherComp :type Primitive%20Component%20Object%20Reference) (OtherBodyIndex :type Integer) (bFromSweep :type Boolean) (SweepResult :type Hit%20Result%20Structure%20%28by%20ref%29))
  (CallFunction|CheckHitCol OtherActor OtherComp))

(event OnComponentBeginOverlap(HitCol)
  (params (OverlappedComponent :type Primitive%20Component%20Object%20Reference) (OtherActor :type Actor%20Object%20Reference) (OtherComp :type Primitive%20Component%20Object%20Reference) (OtherBodyIndex :type Integer) (bFromSweep :type Boolean) (SweepResult :type Hit%20Result%20Structure%20%28by%20ref%29))
  (CallFunction|CheckHitCol OtherActor OtherComp))

(event OnComponentBeginOverlap(HeadCol)
  (params (OverlappedComponent :type Primitive%20Component%20Object%20Reference) (OtherActor :type Actor%20Object%20Reference) (OtherComp :type Primitive%20Component%20Object%20Reference) (OtherBodyIndex :type Integer) (bFromSweep :type Boolean) (SweepResult :type Hit%20Result%20Structure%20%28by%20ref%29))
  (CallFunction|CheckHitCol OtherActor OtherComp))

(event Custom|ShoutPunch
  ;[1 1 1] Shout Inputs
  (Variables|Default|SetShouted_Action "Punch")
  (Variables|Default|SetShout true)
  (Rendering|Components|TextRender|SetText (Variables|Default|GetTextRender) (Utilities|Text|ToText(String) (Variables|Default|GetShouted_Action))))

(event Custom|ShoutPowerAttack
  ;[1 1 1] Shout Inputs
  (Variables|Default|SetShouted_Action "PowerAttack")
  (Variables|Default|SetShout true)
  (Rendering|Components|TextRender|SetText (Variables|Default|GetTextRender) (Utilities|Text|ToText(String) (Variables|Default|GetShouted_Action))))

(event Custom|StaminaGain
  ;[1 1 1] Stress pool Gain
  (if (> (Variables|Default|GetStressPool) (Variables|Default|GetStaminaRegen))
    (Variables|Default|SetStressPool (- (Variables|Default|GetStressPool) (Variables|Default|GetStaminaRegen)))))

(event Custom|DecideAction
  (if (Pawn|IsPlayerControlled)
    ;[1 1 1] Player Shouted
    (if (Variables|Default|GetShout)
      (switch string (Variables|Default|GetDoActionName)
        (:Punch
          (if (Variables|Default|GetFinishedAttack) :!label _label
            (Variables|Default|SetDoActionName (Variables|Default|GetShouted_Action) :!label _label_2)
            (CallFunction|DoAction)
            (else
              (Development|PrintString "WaitingToFinishAnim"))))
        (:Kick
          (goto _label))
        (:Parry
          (goto _label_2))
        (:Block
          (goto _label_2))
        (:Idle
          (goto _label_2))
        (:PowerAttack
          (goto _label)))
      (else
        (if (and (Variables|Default|GetFinishedAttack) (Variables|Default|GetFinishedDefence)) :!label _label_3
          ;[1 1 1] Decide Next Action
          (switch int (Math|Random|RandomInteger 3)
            (:0
              (switch int (Math|Random|RandomInteger 2)
                (:0
                  (Variables|Default|SetDoActionName "Punch"))
                (:1
                  (Variables|Default|SetDoActionName "Kick"))))
            (:1
              (switch int (Math|Random|RandomInteger 2)
                (:0
                  (Variables|Default|SetDoActionName "Parry"))
                (:1
                  (Variables|Default|SetDoActionName "Block"))))
            (:2
              (Variables|Default|SetDoActionName "Idle")))
          (CallFunction|DoAction))))
    (else
      (goto _label_3))))

(event Custom|ShoutKick
  ;[1 1 1] Shout Inputs
  (Variables|Default|SetShouted_Action "Kick")
  (Variables|Default|SetShout true)
  (Rendering|Components|TextRender|SetText (Variables|Default|GetTextRender) (Utilities|Text|ToText(String) (Variables|Default|GetShouted_Action))))

(event Custom|ShoutBlock
  ;[1 1 1] Shout Inputs
  (Variables|Default|SetShouted_Action "Block")
  (Variables|Default|SetShout true)
  (Rendering|Components|TextRender|SetText (Variables|Default|GetTextRender) (Utilities|Text|ToText(String) (Variables|Default|GetShouted_Action))))

(event Custom|DoAction
  ;[1 1 1] Do Action ( AI decided or Shout )
  (Variables|Actions|SetActionIdle false)
  (Variables|Default|SetShout false)
  (switch string (Variables|Default|GetDoActionName)
    (:Punch
      (Variables|Actions|SetActionPunch true)
      (Variables|Default|SetDmgGiven (Variables|Default|GetDmgPunch))
      (Variables|Default|SetFinishedAttack false :!label _label))
    (:Kick
      (Variables|Actions|SetActionKick true)
      (Variables|Default|SetDmgGiven (Variables|Default|GetDmgKick))
      (goto _label))
    (:Parry
      (Variables|Actions|SetActionParry true)
      (Variables|Default|SetFinishedDefence false :!label _label_2))
    (:Block
      (Variables|Actions|SetActionBlock true)
      (goto _label_2))
    (:Idle
      (Variables|Actions|SetActionIdle true))
    (:PowerAttack
      (Variables|Actions|SetActionKick true)
      (Variables|Actions|SetActionPowerAttack true)
      (Variables|Default|SetDmgGiven (Variables|Default|GetDmgPwrAttack))
      (goto _label)))
  (Rendering|Components|TextRender|SetText (Variables|Default|GetTextRender) (Utilities|Text|ToText(String) (Variables|Default|GetDoActionName))))

(event Custom|HitReceived
  ;[1 1 1] Received Hit - Counting it
  (Variables|Default|SetHP (- (Variables|Default|GetHP) (Variables|Default|GetDmgReceived))))

(event EventBeginPlay
  ;[1 1 1] Begin Play - Start timers, Set Stamina
  (Utilities|Time|SetTimerbyFunctionName 0 "DecideAction" 0.1 true)
  (Utilities|Time|SetTimerbyFunctionName 0 "StaminaGain" 1.0 true)
  (Variables|Default|SetHP (Variables|Default|GetHPMax))
  ;[1 1 1] Set Hair Simulation
  (Class|PhysicalAnimationComponent|SetSkeletalMeshComponent (Variables|Default|GetPhysicalAnimation) (Variables|Default|GetHair))
  (Class|SkeletalMeshComponent|SetAllBodiesBelowSimulatePhysics (Variables|Default|GetHair) (Variables|Default|GetHairJoint2Simulate) true true))

(event EventTick
  (params (DeltaSeconds :type Float%20%28single-precision%29))
  ;[1 1 1] Event Tick : Update states
  (Utilities|FlowControl|Sequence
    (:then_0
      (if (Variables|Default|GetFinishedAttack)
        (Variables|Actions|SetActionPunch false)
        (Variables|Actions|SetActionKick false)
        (Variables|Actions|SetActionPowerAttack false)))
    (:then_1
      (if (Variables|Default|GetFinishedDefence)
        (Variables|Actions|SetActionParry false)
        (Variables|Actions|SetActionBlock false)))))

(event Input|ActionEvents|InputActionPunch_1
  (params (Key :type Key%20Structure))
  ;[1 1 1] Shout Inputs
  (:Pressed
    (Variables|Default|SetShouted_Action "Punch")
    (Variables|Default|SetShout true)
    (Rendering|Components|TextRender|SetText (Variables|Default|GetTextRender) (Utilities|Text|ToText(String) (Variables|Default|GetShouted_Action)))))

(event Input|ActionEvents|InputActionGuard_3
  (params (Key :type Key%20Structure))
  ;[1 1 1] Shout Inputs
  (:Pressed
    (Variables|Default|SetShouted_Action "Block")
    (Variables|Default|SetShout true)
    (Rendering|Components|TextRender|SetText (Variables|Default|GetTextRender) (Utilities|Text|ToText(String) (Variables|Default|GetShouted_Action)))))

(event Input|ActionEvents|InputActionKick_2
  (params (Key :type Key%20Structure))
  ;[1 1 1] Shout Inputs
  (:Pressed
    (Variables|Default|SetShouted_Action "Kick")
    (Variables|Default|SetShout true)
    (Rendering|Components|TextRender|SetText (Variables|Default|GetTextRender) (Utilities|Text|ToText(String) (Variables|Default|GetShouted_Action)))))

(fn ConstructionScript)

(fn CheckHitCol
  (params (OtherActor :type Object%20Object%20Reference) (AtherComponent :type Object%20Object%20Reference))
  (bind _returnvalue (Utilities|GetObjectName AtherComponent))
  (if (not (== OtherActor self))
    (if (or (Utilities|Enum|Equal(Enum) _returnvalue "HitCol") (Utilities|Enum|Equal(Enum) _returnvalue "HeadCol"))
      (Variables|Default|SetApplyHit true))))